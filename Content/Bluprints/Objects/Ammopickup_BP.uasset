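; Ammo pickup actor that refills the reserve ammo of the player's weapon when interacted with.
; BeginPlay caches the player character, and a sphere overlap with that character class shows an Interact_WB prompt, removed when the overlap ends.
; The Interact event adds its Ammo value to the weapon's Maxammo, clears any prompt and destroys the pickup.
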(event OnComponentBeginOverlap(Sphere)
  (params (OverlappedComponent :type Primitive%20Component%20Object%20Reference) (OtherActor :type Actor%20Object%20Reference) (OtherComp :type Primitive%20Component%20Object%20Reference) (OtherBodyIndex :type Integer) (bFromSweep :type Boolean) (SweepResult :type Hit%20Result%20Structure%20%28by%20ref%29))
  (Utilities|Casting|CastTofpscharacter_bp OtherActor)
  (bind _returnvalue (UserInterface|CreateWidget "/Game/UI/Interact_WB.Interact_WB_C"))
  (bind _output_get (Variables|Default|Setinteracthud _returnvalue))
  (UserInterface|Viewport|AddtoViewport _output_get 0))

(event OnComponentEndOverlap(Sphere)
  (params (OverlappedComponent :type Primitive%20Component%20Object%20Reference) (OtherActor :type Actor%20Object%20Reference) (OtherComp :type Primitive%20Component%20Object%20Reference) (OtherBodyIndex :type Integer))
  (Utilities|Casting|CastTofpscharacter_bp OtherActor)
  (Utilities|IsValid (Variables|Default|Getinteracthud)
    (:Is%20Valid
      (Widget|RemovefromParent (Variables|Default|Getinteracthud)))))

(event EventBeginPlay
  (bind _asfpscharacter_bp (Utilities|Casting|CastTofpscharacter_bp (Game|GetPlayerCharacter 0)))
  (Variables|Default|SetAs%20Fpscharacter%20Bp _asfpscharacter_bp))

(event Collision|EventActorBeginOverlap
  (params (OtherActor :type Actor%20Object%20Reference)))

(event EventTick
  (params (DeltaSeconds :type Float%20%28single-precision%29)))

(event EventInteract
  (bind _as_fpscharacter_bp (Variables|Default|GetAs%20Fpscharacter%20Bp))
  (bind _interacthud (Variables|Default|Getinteracthud))
  (bind _weaponref (Variables|/Game/blueprints/fpscharacter_bp.fpscharacter_bp_C|Getweaponref _as_fpscharacter_bp))
  (Variables|/Game/blueprints/weapons/Baseweapon_BP.Baseweapon_BP_C|Setmaxammo _weaponref (+ (Variables|/Game/blueprints/weapons/Baseweapon_BP.Baseweapon_BP_C|Getmaxammo _weaponref) (Variables|Default|GetAmmo)))
  (Utilities|IsValid _interacthud
    (:Is%20Valid
      (Widget|RemovefromParent _interacthud)
      (Actor|DestroyActor))
    (:Is%20Not%20Valid
      (Actor|DestroyActor))))

(fn ConstructionScript)