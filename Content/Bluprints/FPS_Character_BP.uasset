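; First-person shooter player character Blueprint that handles movement, look, jumping and weapon fire through Enhanced Input.
; BeginPlay adds the default input mapping context, then caches the ARWEAPON child actor as a BASE_WEAPON_BP and hands it a back-reference to the character.
; Move, look and jump drive the standard character functions, while shoot press and release delegate to the weapon's start and stop shooting calls.
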(event Input|EnhancedActionEvents|EnhancedInputActionIA_LPSP_Movement
  (params (ActionValue :type Vector%202D%20Structure) (ElapsedSeconds :type Float%20%28double-precision%29) (TriggeredSeconds :type Float%20%28double-precision%29) (InputAction :type Input%20Action%20Object%20Reference :default "/Game/InfimaGames/LowPolyShooterPack/Data/Input/IA_LPSP_Movement.IA_LPSP_Movement"))
  ;[1 0.04843 0.8114] handle Movement
  (Pawn|Input|AddMovementInput (Transformation|GetActorRightVector) (.x ActionValue) false)
  (Pawn|Input|AddMovementInput (Transformation|GetActorForwardVector) (.y ActionValue) false))

(event Input|EnhancedActionEvents|EnhancedInputActionIA_LPSP_Look
  (params (ActionValue :type Vector%202D%20Structure) (ElapsedSeconds :type Float%20%28double-precision%29) (TriggeredSeconds :type Float%20%28double-precision%29) (InputAction :type Input%20Action%20Object%20Reference :default "/Game/InfimaGames/LowPolyShooterPack/Data/Input/IA_LPSP_Look.IA_LPSP_Look"))
  ;[0.4077 0.7645 1] Hanfling Look
  (Pawn|Input|AddControllerYawInput (.x ActionValue))
  (Pawn|Input|AddControllerPitchInput (.y ActionValue)))

(event Input|EnhancedActionEvents|EnhancedInputActionIA_LPSP_Jump
  (params (ActionValue :type Boolean) (ElapsedSeconds :type Float%20%28double-precision%29) (TriggeredSeconds :type Float%20%28double-precision%29) (InputAction :type Input%20Action%20Object%20Reference :default "/Game/InfimaGames/LowPolyShooterPack/Data/Input/IA_LPSP_Jump.IA_LPSP_Jump"))
  ;[0.5672 1 0.3543] Handle Jump
  (:Triggered
    (Character|Jump))
  (:Completed
    (Character|StopJumping)))

(event Input|EnhancedActionEvents|EnhancedInputActionIA_LPSP_Shoot
  (params (ActionValue :type Boolean) (ElapsedSeconds :type Float%20%28double-precision%29) (TriggeredSeconds :type Float%20%28double-precision%29) (InputAction :type Input%20Action%20Object%20Reference :default "/Game/InfimaGames/LowPolyShooterPack/Data/Input/IA_LPSP_Shoot.IA_LPSP_Shoot"))
  (bind _weaponref (Variables|Default|Getweaponref))
  (:Started
    (Default|StartShooting _weaponref))
  (:Completed
    (Default|Stopshooting _weaponref)))

(event EventBeginPlay
  ;[0.2997 0.3041 1] Add Input Control
  (bind _asplayer_controller (Utilities|Casting|CastToPlayerController (Pawn|GetController)))
  (Utilities|IsValid (PlayerController|LocalPlayerSubsystems|GetEnhancedInputLocalPlayerSubsystem _asplayer_controller)
    (:Is%20Valid
      (Input|AddMappingContext (PlayerController|LocalPlayerSubsystems|GetEnhancedInputLocalPlayerSubsystem _asplayer_controller) "/Game/InfimaGames/LowPolyShooterPack/Data/Input/IMC_LPSP_Default.IMC_LPSP_Default" 0 "(bIgnoreAllPressedKeysUntilRelease=True,bForceImmediately=False,bNotifyUserSettings=False)")
      (bind _asbase_weapon_bp (Utilities|Casting|CastToBASE_WEAPON_BP (Variables|/Script/Engine.ChildActorComponent|GetChildActor (Variables|Default|GetAR_WEAPON))))
      (bind _output_get (Variables|Default|Setweaponref _asbase_weapon_bp))
      (Variables|/Game/Bluprints/Weapons/BASE_WEAPON_BP.BASE_WEAPON_BP_C|SetPlayerref _output_get self))))

(event Collision|EventActorBeginOverlap
  (params (OtherActor :type Actor%20Object%20Reference)))

(event EventTick
  (params (DeltaSeconds :type Float%20%28single-precision%29)))

(fn ConstructionScript)