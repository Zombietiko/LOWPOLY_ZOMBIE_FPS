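; Rifle weapon Blueprint that handles automatic fire while shooting is active.
; Startshooting fires via Firewesapon and, if Playanimation is true, plays the gun animation and starts a looping Firerate timer.
; Each Firerifle tick fires again, adding the player's first-person hands montage alongside the gun animation.
; The timer clears when Stopshooting is called or a repeat shot finds Playanimation false.
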(event Custom|Firerifle
  (CallFunction|Firewesapon)
  (if (Variables|Default|GetPlayanimation?)
    (Components|Animation|PlayAnimation (Variables|Default|GetGunmesh) "/Game/MilitaryWeapSilver/Weapons/Animations/Fire_Rifle_W.Fire_Rifle_W" false)
    (Animation|Montage|PlayMontage (Variables|/Game/Bluprints/FPS_Charcter_blueprint.FPS_Charcter_blueprint_C|GetFPShands (Variables|Default|GetPlayerref)) "/Game/Content/Man/Demo/Animations/FiringRifle_UE_Montage.FiringRifle_UE_Montage")
    (else
      (Utilities|Time|ClearandInvalidateTimerbyHandle (Variables|Default|GetFireevent)))))

(event EventBeginPlay
  (|CallParentFunction) ; This node is disabled and will not be called.\nDrag off pins to build functionality.
)

(event Collision|EventActorBeginOverlap
  (params (OtherActor :type Actor%20Object%20Reference))
  (|CallParentFunction OtherActor) ; This node is disabled and will not be called.\nDrag off pins to build functionality.
)

(event EventTick
  (params (DeltaSeconds :type Float%20%28single-precision%29))
  (|CallParentFunction DeltaSeconds) ; This node is disabled and will not be called.\nDrag off pins to build functionality.
)

(event EventStartshooting
  (CallFunction|Firewesapon)
  (if (Variables|Default|GetPlayanimation?)
    (Components|Animation|PlayAnimation (Variables|Default|GetGunmesh) "/Game/MilitaryWeapSilver/Weapons/Animations/Fire_Rifle_W.Fire_Rifle_W" false)
    (bind _returnvalue (Utilities|Time|SetTimerbyEvent (delegate Custom|Firerifle) (Variables|Default|GetFirerate) true))
    (Variables|Default|SetFireevent _returnvalue)))

(event EventStopshooting
  (Utilities|Time|ClearandInvalidateTimerbyHandle (Variables|Default|GetFireevent)))

(fn ConstructionScript
  (|CallParentFunction))