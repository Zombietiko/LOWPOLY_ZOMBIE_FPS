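; Assault rifle weapon Blueprint that provides automatic fire while shooting is active.
; StartShooting fires immediately, plays the rifle fire animation on the gun mesh, and starts a looping timer at the fire rate.
; Each timer tick calls FireAR to repeat the shot and animation, and Stopshooting clears the stored timer handle to end the burst.
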(event Custom|FireAR
  (CallFunction|Fireweapon)
  (Components|Animation|PlayAnimation (Variables|Default|GetGunmesh) "/Game/InfimaGames/AnimatedLowPolyWeapons/Art/Characters/Animations/ARs/A_FP_PCH_AR_Fire.A_FP_PCH_AR_Fire" false))

(event EventBeginPlay
  (|CallParentFunction) ; This node is disabled and will not be called.\nDrag off pins to build functionality.
)

(event Collision|EventActorBeginOverlap
  (params (OtherActor :type Actor%20Object%20Reference))
  (|CallParentFunction OtherActor) ; This node is disabled and will not be called.\nDrag off pins to build functionality.
)

(event EventTick
  (params (DeltaSeconds :type Float%20%28single-precision%29))
  (|CallParentFunction DeltaSeconds) ; This node is disabled and will not be called.\nDrag off pins to build functionality.
)

(event EventStartShooting
  (CallFunction|Fireweapon)
  (Components|Animation|PlayAnimation (Variables|Default|GetGunmesh) "/Game/InfimaGames/AnimatedLowPolyWeapons/Art/Characters/Animations/ARs/A_FP_PCH_AR_Fire.A_FP_PCH_AR_Fire" false)
  (bind _returnvalue (Utilities|Time|SetTimerbyEvent (delegate Custom|FireAR) (Variables|Default|GetFirerate) true))
  (Variables|Default|SetFireEvent _returnvalue))

(event EventStopshooting
  (Utilities|Time|ClearandInvalidateTimerbyHandle (Variables|Default|GetFireEvent)))

(fn ConstructionScript
  (|CallParentFunction))