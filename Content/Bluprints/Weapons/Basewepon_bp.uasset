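; Base weapon Blueprint providing hitscan firing, ammo, reloading and iron-sight aiming.
; Firewesapon traces from the player camera, spends a round, sets an animation flag and places a bullet-hole decal, without applying damage.
; Reload refills the magazine from reserve ammo.
; Iron sights blend the view target between weapon and character, with Tick syncing player camera to control rotation while aiming; start/stop shooting events are empty.
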(event Custom|Startshooting)

(event Custom|Stopshooting)

(event Custom|startironsights
  (Variables|Default|SetIronsights true)
  (Game|Player|SetViewTargetwithBlend (Game|GetPlayerController 0) self 0.16 "VTBlend_Linear" 0.0 false))

(event Custom|Stop%20Ironsights
  (Variables|Default|SetIronsights false)
  (Game|Player|SetViewTargetwithBlend (Game|GetPlayerController 0) (Game|GetPlayerCharacter 0) 0.16 "VTBlend_Linear" 0.0 false))

(event EventBeginPlay)

(event Collision|EventActorBeginOverlap
  (params (OtherActor :type Actor%20Object%20Reference)))

(event EventTick
  (params (DeltaSeconds :type Float%20%28single-precision%29))
  (if (Variables|Default|GetIronsights)
    (Transformation|SetWorldRotation (Variables|/Game/Bluprints/FPS_Charcter_blueprint.FPS_Charcter_blueprint_C|GetCamera (Variables|Default|GetPlayerref)) (Pawn|GetControlRotation (Game|GetPlayerController 0) :!class /Script/Engine.Controller) false false)))

(fn ConstructionScript)

(fn Firewesapon
  (bind _playerref (Variables|Default|GetPlayerref))
  (bind _camera (Variables|/Game/Bluprints/FPS_Charcter_blueprint.FPS_Charcter_blueprint_C|GetCamera _playerref))
  (bind _returnvalue (Transformation|GetWorldLocation _camera))
  (if (> (Variables|Default|GetCurrentammo) 0)
    (Variables|Default|SetPlayanimation? true)
    (bind _outhit (Collision|LineTraceByChannel _returnvalue (+ _returnvalue (* (Math|Vector|GetForwardVector _camera) 3e+03)) "TraceTypeQuery1" false 0 "None"))
    (Math|Integer|DecrementInt (Variables|Default|GetCurrentammo)
      (:%20%20
        (Rendering|Decal|SpawnDecalatLocation "/Game/Images/bullet_hole_Mat.bullet_hole_Mat" "6.000000,6.000000,6.000000" (.Location (Collision|BreakHitResult _outhit)) (Math|Conversions|RotationFromXVector (.ImpactNormal (Collision|BreakHitResult _outhit))) 5.0)))
    (else
      (Variables|Default|SetPlayanimation? false))))

(fn Reload
  (bind _output_get (LocalVariables|SetAmmodifference (- (Variables|Default|GetMagazinesize) (Variables|Default|GetCurrentammo))))
  (if (>= (Variables|Default|GetMaxammo) _output_get)
    (Variables|Default|SetCurrentammo (Variables|Default|GetMagazinesize))
    (Variables|Default|SetMaxammo (- (Variables|Default|GetMaxammo) (LocalVariables|GetAmmodifference)))
    (else
      (Variables|Default|SetCurrentammo (+ (Variables|Default|GetCurrentammo) (Variables|Default|GetMaxammo)))
      (Variables|Default|SetMaxammo 0))))