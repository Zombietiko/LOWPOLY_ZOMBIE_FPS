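; Shotgun weapon Blueprint that handles the shooting event with shotgun-specific animation.
; Startshooting calls Firewesapon, whose logic is not defined in this graph, then checks the Playanimation flag.
; When the flag is set, it plays the shotgun fire animation on the gun mesh and a rifle firing montage on the player's first-person hands.
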(event EventBeginPlay
  (|CallParentFunction) ; This node is disabled and will not be called.\nDrag off pins to build functionality.
)

(event Collision|EventActorBeginOverlap
  (params (OtherActor :type Actor%20Object%20Reference))
  (|CallParentFunction OtherActor) ; This node is disabled and will not be called.\nDrag off pins to build functionality.
)

(event EventTick
  (params (DeltaSeconds :type Float%20%28single-precision%29))
  (|CallParentFunction DeltaSeconds) ; This node is disabled and will not be called.\nDrag off pins to build functionality.
)

(event EventStartshooting
  (CallFunction|Firewesapon)
  (if (Variables|Default|GetPlayanimation?)
    (Components|Animation|PlayAnimation (Variables|Default|GetGunmesh) "/Game/MilitaryWeapSilver/Weapons/Animations/Fire_Shotgun_W.Fire_Shotgun_W" false)
    (Animation|Montage|PlayMontage (Variables|/Game/Bluprints/FPS_Charcter_blueprint.FPS_Charcter_blueprint_C|GetFPShands (Variables|Default|GetPlayerref)) "/Game/Content/Man/Demo/Animations/FiringRifle_UE_Montage.FiringRifle_UE_Montage")))

(fn ConstructionScript
  (|CallParentFunction))