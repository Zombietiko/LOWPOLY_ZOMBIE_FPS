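; Weapon pickup actor that swaps its stored weapon and ammo with the FPS player character's currently held weapon.
; On Interact, it checks whether the main or secondary slot is equipped and spawns a new pickup holding that slot's weapon.
; It then writes itself into the slot, changes the character's weapon child actor, refreshes HUD and ammo, and destroys itself.
; The construction script picks the pistol, rifle or shotgun mesh from the weapon class's default name.
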(event EventBeginPlay
  (bind _asfps_charcter_blueprint (Utilities|Casting|CastToFPS_Charcter_blueprint (Game|GetPlayerCharacter 0)))
  (Variables|Default|SetAs%20FPS%20Charcter%20Blueprint _asfps_charcter_blueprint))

(event Collision|EventActorBeginOverlap
  (params (OtherActor :type Actor%20Object%20Reference)))

(event EventTick
  (params (DeltaSeconds :type Float%20%28single-precision%29)))

(event EventInteract
  (bind _as_fps_charcter_blueprint (Variables|Default|GetAs%20FPS%20Charcter%20Blueprint))
  (bind _as_fps_charcter_blueprint_2 (Variables|Default|GetAs%20FPS%20Charcter%20Blueprint))
  (bind _weapon (Variables|Default|GetWeapon))
  (bind _weapon_2 (Variables|Default|GetWeapon))
  (bind _as_fps_charcter_blueprint_3 (Variables|Default|GetAs%20FPS%20Charcter%20Blueprint))
  (bind _as_fps_charcter_blueprint_4 (Variables|Default|GetAs%20FPS%20Charcter%20Blueprint))
  (bind _weapon_3 (Variables|Default|GetWeapon))
  (bind _weapon_4 (Variables|Default|GetWeapon))
  (bind _as_fps_charcter_blueprint_5 (Variables|Default|GetAs%20FPS%20Charcter%20Blueprint))
  (bind _weaponref (Variables|/Game/Bluprints/FPS_Charcter_blueprint.FPS_Charcter_blueprint_C|GetWeaponref _as_fps_charcter_blueprint_2))
  (bind _weaponref_2 (Variables|/Game/Bluprints/FPS_Charcter_blueprint.FPS_Charcter_blueprint_C|GetWeaponref _as_fps_charcter_blueprint_4))
  (if (== (Variables|/Script/Engine.ChildActorComponent|GetChildActorClass (Variables|/Game/Bluprints/FPS_Charcter_blueprint.FPS_Charcter_blueprint_C|GetWeapon _as_fps_charcter_blueprint)) (.weapon (Variables|/Game/Bluprints/FPS_Charcter_blueprint.FPS_Charcter_blueprint_C|GetMainweapon _as_fps_charcter_blueprint)))
    (Game|SpawnActorfromClass "Weaponpickup_bp_C" (Transformation|GetActorTransform) "Undefined" "MultiplyWithRoot" 0 (Variables|/Game/Bluprints/FPS_Charcter_blueprint.FPS_Charcter_blueprint_C|GetMainweapon (Variables|Default|GetAs%20FPS%20Charcter%20Blueprint)) 0)
    (Variables|/Game/Bluprints/FPS_Charcter_blueprint.FPS_Charcter_blueprint_C|SetMainweapon (Variables|Default|GetAs%20FPS%20Charcter%20Blueprint) (Utilities|Struct|MakeWeaponsruct (.weapon _weapon_2) (.currentammo _weapon_2) (.maxammo _weapon_2)))
    (Widget|RemovefromParent (Variables|/Game/Bluprints/FPS_Charcter_blueprint.FPS_Charcter_blueprint_C|GetPlayerhudref _as_fps_charcter_blueprint_3))
    (ChildActorComponent|SetChildActorClass (Variables|/Game/Bluprints/FPS_Charcter_blueprint.FPS_Charcter_blueprint_C|GetWeapon _as_fps_charcter_blueprint_3) (.weapon (Variables|Default|GetWeapon)))
    (Default|Update (Variables|Default|GetAs%20FPS%20Charcter%20Blueprint))
    (Variables|/Game/Bluprints/Weapons/Basewepon_bp.Basewepon_bp_C|SetCurrentammo _weaponref_2 (.currentammo _weapon_3))
    (Variables|/Game/Bluprints/Weapons/Basewepon_bp.Basewepon_bp_C|SetMaxammo _weaponref_2 (.maxammo _weapon_3))
    (Actor|DestroyActor)
    (else
      (Game|SpawnActorfromClass "Weaponpickup_bp_C" (Transformation|GetActorTransform) "Undefined" "MultiplyWithRoot" 0 (Variables|/Game/Bluprints/FPS_Charcter_blueprint.FPS_Charcter_blueprint_C|GetSecondaryweapon (Variables|Default|GetAs%20FPS%20Charcter%20Blueprint)) 0)
      (Variables|/Game/Bluprints/FPS_Charcter_blueprint.FPS_Charcter_blueprint_C|SetSecondaryweapon (Variables|Default|GetAs%20FPS%20Charcter%20Blueprint) (Utilities|Struct|MakeWeaponsruct (.weapon _weapon_4) (.currentammo _weapon_4) (.maxammo _weapon_4)))
      (Widget|RemovefromParent (Variables|/Game/Bluprints/FPS_Charcter_blueprint.FPS_Charcter_blueprint_C|GetPlayerhudref _as_fps_charcter_blueprint_5))
      (ChildActorComponent|SetChildActorClass (Variables|/Game/Bluprints/FPS_Charcter_blueprint.FPS_Charcter_blueprint_C|GetWeapon _as_fps_charcter_blueprint_5) (.weapon (Variables|Default|GetWeapon)))
      (Default|Update (Variables|Default|GetAs%20FPS%20Charcter%20Blueprint))
      (Variables|/Game/Bluprints/Weapons/Basewepon_bp.Basewepon_bp_C|SetCurrentammo _weaponref (.currentammo _weapon))
      (Variables|/Game/Bluprints/Weapons/Basewepon_bp.Basewepon_bp_C|SetMaxammo _weaponref (.maxammo _weapon))
      (Actor|DestroyActor))))

(fn ConstructionScript
  (switch string (Utilities|String|ToString(Text) (.Weaponname (Utilities|GetClassDefaults (.weapon (Variables|Default|GetWeapon)))))
    (:Pistol
      (Components|SkeletalMesh|SetSkeletalMeshAsset (Variables|Default|GetSkeletalMesh) "/Game/MilitaryWeapSilver/Weapons/Pistols_A.Pistols_A"))
    (:Rifle
      (Components|SkeletalMesh|SetSkeletalMeshAsset (Variables|Default|GetSkeletalMesh) "/Game/MilitaryWeapSilver/Weapons/Assault_Rifle_A.Assault_Rifle_A"))
    (:Shotgun
      (Components|SkeletalMesh|SetSkeletalMeshAsset (Variables|Default|GetSkeletalMesh) "/Game/MilitaryWeapSilver/Weapons/Shotgun_A.Shotgun_A"))))