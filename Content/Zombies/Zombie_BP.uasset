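; Zombie character Blueprint that wanders at random and chases pawns it sees.
; BeginPlay sets walk speed from ZombieSpeed and starts Roam, which moves to random reachable points nearby and repeats after each successful move while no pawn is seen.
; PawnSensing sightings start an AI move toward the pawn and set Seesplayer.
; A retriggerable delay clears that flag and resumes roaming a few seconds after the last sighting.
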(event OnSeePawn(PawnSensing)
  (params (Pawn :type Pawn%20Object%20Reference))
  (Variables|Default|Setseesplayer true)
  (Utilities|FlowControl|Sequence
    (:then_0
      (AI|AIMoveTo self "0, 0, 0" Pawn 5.0 false))
    (:then_1
      (Utilities|FlowControl|RetriggerableDelay 3.0)
      (Variables|Default|Setseesplayer false)
      (CallFunction|Roam))))

(event Custom|Roam
  (if (not (Variables|Default|Getseesplayer)) :!label _label
    (AI|AIMoveTo self (.RandomLocation (AI|Navigation|GetRandomReachablePointinRadius (Transformation|GetActorLocation) 5e+02 0 0)) 0 5.0 false
      (:OnSuccess
        (Utilities|FlowControl|Delay 0.2)
        (goto _label)))))

(event EventBeginPlay
  (Variables|/Script/Engine.CharacterMovementComponent|SetMaxWalkSpeed (Variables|Character|GetCharacterMovement) (Variables|Default|GetZombieSpeed))
  (CallFunction|Roam))

(event Collision|EventActorBeginOverlap
  (params (OtherActor :type Actor%20Object%20Reference)))

(event EventTick
  (params (DeltaSeconds :type Float%20%28single-precision%29)))

(fn ConstructionScript)